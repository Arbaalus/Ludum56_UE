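; Mini-boss turtle tank enemy that fires twin cannons at the player and shows the Level 2 transition widget when it dies.
; Looping timers turn the tank base toward the player and fire each cannon after a random delay, unless IsReadyToCharge is set.
; Two timelines restart each other to swing the jaw mesh continuously.
; Damage arrives through an interface event, with attached audio for shots, hits and death.
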(event `self.ReceiveBeginPlay`
  (`parent.ReceiveBeginPlay`)
  (`KismetSystemLibrary.K2_SetTimerDelegate` (delegate `TargetPlayer`) 0.05 true)
  (`KismetSystemLibrary.K2_SetTimerDelegate` (delegate `ShootPlayerWithCannonRight`) 1.5 true)
  (`KismetSystemLibrary.K2_SetTimerDelegate` (delegate `ShootPlayerWithCannonLeft`) 1.5 true)
  (bind (_direction _alpha) (`Timeline|Timeline` :!via `PlayFromStart` :!label _label)
    (:`Update`
      (`SceneComponent.K2_SetRelativeRotation` (`self.M_TankTortue__Machoire`) (`KismetMathLibrary.MakeRotator` 0.0 (`KismetMathLibrary.Lerp` 4.0 -20.0 _alpha)) false false))
    (:`Finished`
      (bind (_direction_2 _alpha_2) (`Timeline|Timeline_0` :!via `PlayFromStart`)
        (:`Update`
          (`SceneComponent.K2_SetRelativeRotation` (`self.M_TankTortue__Machoire`) (`KismetMathLibrary.MakeRotator` 0.0 (`KismetMathLibrary.Lerp` -20.0 4.0 _alpha_2)) false false))
        (:`Finished`
          (goto _label :!via `PlayFromStart`))))))

(event `TargetPlayer`
  (`SceneComponent.K2_SetWorldRotation` (`self.M_Tank__Base`) (`KismetMathLibrary.FindLookAtRotation` (`SceneComponent.K2_GetComponentLocation` (`self.M_Tank__Base`)) (`self.K2_GetActorLocation` (`GameplayStatics.GetPlayerCharacter` 0))) false false))

(event `ShootPlayerWithCannonRight`
  (if (not (`self.IsReadyToCharge`))
    (`KismetSystemLibrary.Delay` (`KismetMathLibrary.RandomFloatInRange` 0.0 1.5))
    (`|SpawnActorFromClass` "/Game/BluePrint/EnemyProjectileBase.EnemyProjectileBase_C" (`SceneComponent.K2_GetComponentToWorld` (`self.TourelleArrowRight`)) "AlwaysSpawn" "MultiplyWithRoot" null (`self.ProjectileSpeed`) null)
    (`FMODBlueprintStatics.PlayEventAttached` "/Game/FMOD/Events/SFX_TurtleTank_Gun.SFX_TurtleTank_Gun" (`self.CapsuleComponent`) "None" (0.0 0.0 0.0) "KeepRelativeOffset" :!label _label_2)))

(event `ShootPlayerWithCannonLeft`
  (if (not (`self.IsReadyToCharge`))
    (`KismetSystemLibrary.Delay` (`KismetMathLibrary.RandomFloatInRange` 0.0 1.5))
    (`|SpawnActorFromClass` "/Game/BluePrint/EnemyProjectileBase.EnemyProjectileBase_C" (`SceneComponent.K2_GetComponentToWorld` (`self.TourelleArrowRightLeft`)) "AlwaysSpawn" "MultiplyWithRoot" null (`self.ProjectileSpeed`) null)
    (goto _label_2)))

(event `self.BPI_enemyTakeDamage`
  (params (dmg :type Integer))
  (`self.TakeDamage` dmg)
  (`FMODBlueprintStatics.PlayEventAttached` "/Game/FMOD/Events/VX_Boss_Hit.VX_Boss_Hit" (`self.CapsuleComponent`) "None" (0.0 0.0 0.0) "KeepRelativeOffset"))

(fn `Die`
  (`FMODBlueprintStatics.PlayEventAttached` "/Game/FMOD/Events/VX_Boss_Death.VX_Boss_Death" (`self.CapsuleComponent`) "None" (0.0 0.0 0.0) "KeepRelativeOffset")
  (bind _returnvalue (`|CreateWidget` "/Game/BluePrint/UI/TransitionLevel2.TransitionLevel2_C"))
  (`UserWidget.AddToViewport` _returnvalue 0)
  (`parent.Die`))

(fn `UserConstructionScript`
  (`parent.UserConstructionScript`))