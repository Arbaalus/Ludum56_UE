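; AI controller logic for an enemy mini-boss that keeps a distance band from the player.
; A half-second looping timer compares the pawn's distance to player 0, stepping away when too close and closer when too far via short AIMoveTo offsets along the look-at direction, flattened horizontally.
; BeginPlay also attaches a looping-timer-independent engine sound to the pawn; the move branches print debug text and call PlayEventAttached with no event assigned.
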(event `self.ReceiveBeginPlay`
  (bind _returnvalue (`self.K2_GetPawn`))
  (`KismetSystemLibrary.K2_SetTimerDelegate` :`Time` 1.0)
  (`KismetSystemLibrary.K2_SetTimerDelegate` (delegate `MoveWithPLayer`) 0.5 true)
  (`/Engine/EditorBlueprintResources/StandardMacros.IsValid` _returnvalue
    (:`Is Valid`
      (`FMODBlueprintStatics.PlayEventAttached` "/Game/FMOD/Events/SFX_Boss_Engine.SFX_Boss_Engine" (`Actor.RootComponent` _returnvalue) "None" (0.0 0.0 0.0) "KeepRelativeOffset" true))))

(event `MoveWithPLayer`
  (bind _returnvalue (`self.K2_GetPawn`))
  (bind _returnvalue_2 (`GameplayStatics.GetPlayerCharacter` 0))
  (bind _returnvalue_3 (`self.K2_GetActorLocation` _returnvalue))
  (bind _returnvalue_4 (`self.GetDistanceTo` _returnvalue _returnvalue_2))
  (bind _returnvalue_5 (`KismetMathLibrary.GetForwardVector` (`KismetMathLibrary.FindLookAtRotation` _returnvalue_3 (`self.K2_GetActorLocation` _returnvalue_2))))
  (if (< _returnvalue_4 1100.0)
    (`|AIMoveTo` null (+ _returnvalue_3 (* _returnvalue_5 (-300.0 -300.0 0.0))) null
      (:`then`
        (`KismetSystemLibrary.PrintString` "away from player")
        (`FMODBlueprintStatics.PlayEventAttached` null null "None" _returnvalue_3 "KeepRelativeOffset" :!label _label)))
    (elif (> _returnvalue_4 1400.0)
      (`|AIMoveTo` null (+ _returnvalue_3 (* _returnvalue_5 (200.0 200.0 0.0))) null
        (:`then`
          (`KismetSystemLibrary.PrintString` "Moving near player")
          (goto _label))))))

(fn `UserConstructionScript`)