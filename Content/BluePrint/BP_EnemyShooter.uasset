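; BP_EnemyShooter is an enemy turret that aims at the player and fires projectiles.
; Two looping timers start on BeginPlay: a fast one turns the Tourelle component toward the player character, and a slower one triggers shooting.
; Each shot waits a random delay to vary its timing, then spawns an EnemyProjectileBase at the TourelleArrow transform with the turret's ProjectileSpeed.
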(event `self.ReceiveBeginPlay`
  (`parent.ReceiveBeginPlay`)
  (`KismetSystemLibrary.K2_SetTimerDelegate` (delegate `TargetPlayer`) 0.05 true)
  (`KismetSystemLibrary.K2_SetTimerDelegate` (delegate `ShootPlayer`) 3.0 true))

(event `TargetPlayer`
  (`SceneComponent.K2_SetWorldRotation` (`self.Tourelle`) (`KismetMathLibrary.FindLookAtRotation` (`SceneComponent.K2_GetComponentLocation` (`self.Tourelle`)) (`self.K2_GetActorLocation` (`GameplayStatics.GetPlayerCharacter` 0))) false false))

(event `ShootPlayer`
  (`KismetSystemLibrary.Delay` (`KismetMathLibrary.RandomFloatInRange` 0.0 2.0))
  (`|SpawnActorFromClass` "/Game/BluePrint/EnemyProjectileBase.EnemyProjectileBase_C" (`SceneComponent.K2_GetComponentToWorld` (`self.TourelleArrow`)) "AlwaysSpawn" "MultiplyWithRoot" null (`self.ProjectileSpeed`) null))

(fn `UserConstructionScript`
  (`parent.UserConstructionScript`))