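; Flying AI seagull that dive-chases the player, drops an egg over them, then leaves and despawns.
; Tick drives the AI controller toward the player without pathfinding, playing a one-shot drive-by sound on approach.
; Once within close range, it spawns an egg high at the player's XY, numbered by the parent area's counter.
; It then heads to an externally set end location and destroys itself on arrival.
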(event `self.ReceiveBeginPlay`
  (bind _charactermovement (`self.CharacterMovement`))
  (`CharacterMovementComponent.SetMovementMode` _charactermovement "MOVE_Flying" 0)
  (set `CharacterMovementComponent.MaxFlySpeed` 2000.0 _charactermovement)
  (`KismetSystemLibrary.K2_SetTimerDelegate` (`|CreateDelegate` :!event `UpdateInfos`) 1.0 true))

(event `self.ReceiveTick`
  (params (DeltaSeconds :type "Float (single-precision)"))
  (bind _endreached (`self.IsEndReached`))
  (if (not _endreached)
    (bind _playerreached (`self.IsPlayerReached`))
    (if _playerreached
      (`self.MoveToEnd`)
      (else
        (`self.IsPlayerNear`)
        (`self.MoveToPlayer`)))))

(event `UpdateInfos`)

(fn `IsEndReached`
  (returns (EndReached :type Boolean))
  (if (< (`KismetMathLibrary.Vector_Distance` (`self.K2_GetActorLocation` self) (`self.EndLocation`)) 100.0)
    (`self.K2_DestroyActor` self)
    (return true)
    (else
      (return false))))

(fn `IsPlayerNear`
  (if (`self.SeagullScreamDone`)
    (return)
    (elif (< (`KismetMathLibrary.Vector_Distance` (`self.K2_GetActorLocation` self) (`self.K2_GetActorLocation` (`GameplayStatics.GetPlayerPawn` 0))) 3000.0)
      (`FMODBlueprintStatics.PlayEventAttached` "/Game/FMOD/Events/SFX_Seagull_DriveBy.SFX_Seagull_DriveBy" (`self.CapsuleComponent`) "None" (0.0 0.0 0.0) "KeepRelativeOffset")
      (set `self.SeagullScreamDone` true)
      (return)
      (else
        (return)))))

(fn `IsPlayerReached`
  (returns (PlayerReached :type Boolean))
  (if (`self.ReachedPlayer`)
    (return true)
    (elif (< (`KismetMathLibrary.Vector_Distance` (`self.K2_GetActorLocation` self) (`self.K2_GetActorLocation` (`GameplayStatics.GetPlayerPawn` 0))) 300.0)
      (set `self.ReachedPlayer` true)
      (`self.SpawnEgg`)
      (return true)
      (else
        (return false)))))

(fn `MoveToEnd`
  (`AIController.MoveToLocation` (`AIBlueprintHelperLibrary.GetAIController` self) (`self.EndLocation`) 1.0 true false false true null true))

(fn `MoveToPlayer`
  (`AIController.MoveToLocation` (`AIBlueprintHelperLibrary.GetAIController` self) (`self.K2_GetActorLocation` (`GameplayStatics.GetPlayerPawn` 0)) 1.0 true false false true null true))

(fn `SetEndLocation`
  (params (NewEndLocation :type "Vector Structure"))
  (set `self.EndLocation` NewEndLocation))

(fn `SetParentArea`
  (params (NewParentArea :type "/Game/BluePrint/BP_SeagullArea Object Reference"))
  (set `self.ParentArea` NewParentArea))

(fn `SetSeagullId`
  (params (SeagullId :type Integer))
  (set `self.SeagullId` SeagullId))

(fn `SpawnEgg`
  (bind _parentarea (`self.ParentArea`))
  (bind (_returnvalue_x _returnvalue_y) (`KismetMathLibrary.BreakVector` (`self.K2_GetActorLocation` (`GameplayStatics.GetPlayerPawn` 0))))
  (bind _returnvalue (`|SpawnActorFromClass` "/Game/BluePrint/BP_SeagullEggActor.BP_SeagullEggActor_C" (`KismetMathLibrary.MakeTransform` (`KismetMathLibrary.MakeVector` _returnvalue_x _returnvalue_y 2000.0)) "AlwaysSpawn" "MultiplyWithRoot" null null))
  (bind _eggspawnedcounter (`/Game/BluePrint/BP_SeagullArea.GetEggSpawnedCounter` _parentarea))
  (`/Game/BluePrint/BP_SeagullEggActor.SetEggId` _returnvalue _eggspawnedcounter)
  (`/Game/BluePrint/BP_SeagullArea.IncrementEggSpawnedCounter` _parentarea))

(fn `UserConstructionScript`)