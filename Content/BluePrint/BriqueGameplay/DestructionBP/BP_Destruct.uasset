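; Destructible Chaos Geometry Collection actor that collapses with sound and removes itself after breaking.
; On the Chaos break event, it plays the collapse SFX once, makes the collection dynamic, disables the Box collision and destroys the actor 20 seconds later.
; The hit handler is empty, and the impact-threshold, field-spawning and explosion logic is disconnected, leaving the delayed DestructionOn flag without effect.
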(event `self.ReceiveBeginPlay`
  (`KismetSystemLibrary.Delay` 1.0)
  (set `self.DestructionOn` true))

(event `self.GC_Cube.OnComponentHit`
  (params (HitComponent :type "PrimitiveComponent Object Reference") (OtherActor :type "Actor Object Reference") (OtherComp :type "PrimitiveComponent Object Reference") (NormalImpulse :type "Vector Structure") (Hit :type "HitResult Structure (by ref)")))

(event `self.GC_Cube.OnChaosBreakEvent`
  (params (BreakEvent :type "ChaosBreakEvent Structure (by ref)"))
  (`|ExecutionSequence`
    (:`then_0`
      (`/Engine/EditorBlueprintResources/StandardMacros.DoOnce` false
        (:`Completed`
          (`FMODBlueprintStatics.PlayEventAtLocation` "/Game/FMOD/Events/SFX_Collapse.SFX_Collapse" (`KismetMathLibrary.Conv_VectorToTransform` (`self.K2_GetActorLocation`))))))
    (:`then_1`
      (set `GeometryCollectionComponent.ObjectType` "Chaos_Object_Dynamic" (`self.GC_Cube`))
      (`PrimitiveComponent.SetCollisionEnabled` (`self.Box`) "NoCollision")
      (`KismetSystemLibrary.Delay` 20.0)
      (`self.K2_DestroyActor`))))

(fn `UserConstructionScript`)