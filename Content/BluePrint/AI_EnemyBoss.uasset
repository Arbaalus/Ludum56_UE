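; AI controller for the enemy boss that alternates between spacing itself from the player and charge attacks, without a behavior tree.
; A looping timer steps it via AIMoveTo toward the player when ready to charge, or holds a distance band during cooldown.
; Within range, it pauses to telegraph, boosts walk speed and launches the character, then restarts the cooldown.
; It also plays an attached engine sound.
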(event `self.ReceiveBeginPlay`
  (bind _asbp_enemy_boss (cast `/Game/BluePrint/BP_EnemyBoss` (`self.K2_GetPawn`)))
  (bind _output_get (set `self.BossReference` _asbp_enemy_boss))
  (set `self.BaseMaxWalkSpeed` (`CharacterMovementComponent.MaxWalkSpeed` (`Character.CharacterMovement` _output_get)))
  (`KismetSystemLibrary.K2_SetTimerDelegate` (delegate `StartChargeCooldown`) 1.0)
  (`KismetSystemLibrary.K2_SetTimerDelegate` (delegate `MoveWithPLayer`) 0.5 true)
  (`FMODBlueprintStatics.PlayEventAttached` "/Game/FMOD/Events/SFX_Boss_Engine.SFX_Boss_Engine" (`Actor.RootComponent` (`self.K2_GetPawn`)) "None" (0.0 0.0 0.0) "KeepRelativeOffset"))

(event `MoveWithPLayer`
  (bind _returnvalue (`self.K2_GetPawn`))
  (bind (_returnvalue_x _returnvalue_y) (`KismetMathLibrary.BreakVector` (`KismetMathLibrary.Vector_Forward`)))
  (bind _returnvalue_2 (`GameplayStatics.GetPlayerCharacter` 0))
  (bind _bossreference (`self.BossReference`))
  (bind _returnvalue_3 (`self.K2_GetActorLocation` _returnvalue))
  (bind _returnvalue_4 (`self.GetDistanceTo` _returnvalue _returnvalue_2))
  (bind _charactermovement (`Character.CharacterMovement` _bossreference))
  (bind _returnvalue_5 (`KismetMathLibrary.GetForwardVector` (`KismetMathLibrary.FindLookAtRotation` _returnvalue_3 (`self.K2_GetActorLocation` _returnvalue_2))))
  (if (`/Game/BluePrint/BP_EnemyBoss.IsReadyToCharge` (`self.BossReference`))
    (if (< _returnvalue_4 1000.0)
      (if (not (`self.IsCharging`))
        (set `self.IsCharging` true)
        (`KismetSystemLibrary.PrintString` "Le boss a un effet de charge d'attaque")
        (`KismetSystemLibrary.Delay` 1.5)
        (set `CharacterMovementComponent.MaxWalkSpeed` 1500.0 _charactermovement)
        (`Character.LaunchCharacter` _bossreference (`KismetMathLibrary.MakeVector` (* _returnvalue_x 3000.0) (* _returnvalue_y 3000.0)) true true)
        (`KismetSystemLibrary.Delay` 1.0)
        (set `/Game/BluePrint/BP_EnemyBoss.IsReadyToCharge` false _bossreference)
        (set `self.IsCharging` false)
        (`self.StartChargeCooldown`)
        (set `CharacterMovementComponent.MaxWalkSpeed` (`self.BaseMaxWalkSpeed`) _charactermovement))
      (else
        (`|AIMoveTo` null (+ _returnvalue_3 (* _returnvalue_5 (200.0 200.0 0.0))) null :!label _label
          (:`then`
            (`KismetSystemLibrary.PrintString` "Moving near player")
            (`FMODBlueprintStatics.PlayEventAttached` null null "None" _returnvalue_3 "KeepRelativeOffset" :!label _label_2)))))
    (elif (< _returnvalue_4 1200.0)
      (`|AIMoveTo` null (+ _returnvalue_3 (* _returnvalue_5 (-300.0 -300.0 0.0))) null
        (:`then`
          (`KismetSystemLibrary.PrintString` "away from player")
          (goto _label_2)))
      (elif (> _returnvalue_4 1400.0)
        (goto _label)))))

(event `StartChargeCooldown`
  (`KismetSystemLibrary.Delay` (`self.ChargeCooldown`))
  (set `/Game/BluePrint/BP_EnemyBoss.IsReadyToCharge` true (`self.BossReference`))
  (`KismetSystemLibrary.PrintString` "Boss is ready to charge ! "))

(fn `UserConstructionScript`)