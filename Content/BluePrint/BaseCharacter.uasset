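; BaseCharacter is a Blueprint, named as a character base, that provides simple health and death handling.
; BeginPlay fills CurrentHealth from MaxHealth, and the custom TakeDamage function subtracts incoming damage from it.
; When health reaches zero or below, TakeDamage calls Die, which prints a message and destroys the actor.
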(event `self.ReceiveBeginPlay`
  (set `self.CurrentHealth` (`self.MaxHealth`)))

(fn `Die`
  (`KismetSystemLibrary.PrintString` "Someone died")
  (`self.K2_DestroyActor`))

(fn `TakeDamage`
  (params (Damage :type Integer))
  (bind _output_get (set `self.CurrentHealth` (- (`self.CurrentHealth`) Damage)))
  (if (<= _output_get 0)
    (`self.Die`)))

(fn `UserConstructionScript`)