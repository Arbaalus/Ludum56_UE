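; BP_EnemyBoss is a boss enemy with a tracking turret and two cannons, built on a parent enemy class.
; On BeginPlay, looping timers keep the turret rotated toward player 0 and trigger both cannons.
; Each cannon waits a random delay, then spawns an EnemyProjectileBase from its mesh transform, unless IsReadyToCharge is set.
; Die plays an attached death sound or effect event and shows the LoseScreen widget before calling the parent Die.
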(event `self.ReceiveBeginPlay`
  (`parent.ReceiveBeginPlay`)
  (`KismetSystemLibrary.K2_SetTimerDelegate` (delegate `TargetPlayer`) 0.05 true)
  (`KismetSystemLibrary.K2_SetTimerDelegate` (delegate `ShootPlayerLeftCanon`) 2.0 true)
  (`KismetSystemLibrary.K2_SetTimerDelegate` (delegate `ShootPlayerRightCanon`) 2.0 true))

(event `TargetPlayer`
  (`SceneComponent.K2_SetWorldRotation` (`self.Tourelle`) (`KismetMathLibrary.FindLookAtRotation` (`SceneComponent.K2_GetComponentLocation` (`self.Tourelle`)) (`self.K2_GetActorLocation` (`GameplayStatics.GetPlayerCharacter` 0))) false false))

(event `ShootPlayerRightCanon`
  (if (not (`self.IsReadyToCharge`))
    (`KismetSystemLibrary.Delay` (`KismetMathLibrary.RandomFloatInRange` 0.0 2.0))
    (`|SpawnActorFromClass` "/Game/BluePrint/EnemyProjectileBase.EnemyProjectileBase_C" (`SceneComponent.K2_GetComponentToWorld` (`self.M_TankTortue__Base2`)) "AlwaysSpawn" "MultiplyWithRoot" null (`self.ProjectileSpeed`) null)))

(event `ShootPlayerLeftCanon`
  (if (not (`self.IsReadyToCharge`))
    (`KismetSystemLibrary.Delay` (`KismetMathLibrary.RandomFloatInRange` 0.0 2.0))
    (`|SpawnActorFromClass` "/Game/BluePrint/EnemyProjectileBase.EnemyProjectileBase_C" (`SceneComponent.K2_GetComponentToWorld` (`self.M_TankTortue__Base1`)) "AlwaysSpawn" "MultiplyWithRoot" null (`self.ProjectileSpeed`) null)))

(fn `Die`
  (`FMODBlueprintStatics.PlayEventAttached` "/Game/FMOD/Events/VX_Boss_Death.VX_Boss_Death" (`self.CapsuleComponent`) "None" (0.0 0.0 0.0) "SnapToTargetIncludingScale")
  (bind _returnvalue (`|CreateWidget` "/Game/BluePrint/UI/LoseScreen.LoseScreen_C"))
  (`UserWidget.AddToViewport` _returnvalue 0)
  (`parent.Die`))

(fn `UserConstructionScript`
  (`parent.UserConstructionScript`))