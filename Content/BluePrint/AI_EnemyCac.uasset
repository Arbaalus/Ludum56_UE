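; AI controller for a melee enemy that sends its pawn toward the player character.
; A looping one-second timer issues an AI MoveTo when the distance between the pawn and the controller itself, not the player, is under the aggro threshold.
; Each move request immediately plays two turtle footstep events attached to the pawn, separated by a short delay.
; Otherwise it prints that distance for debugging.
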(event `self.ReceiveBeginPlay`
  (`KismetSystemLibrary.K2_SetTimerDelegate` (delegate `TrackPlayer`) 1.0 true))

(event `TrackPlayer`
  (bind _returnvalue (`self.K2_GetPawn`))
  (bind _returnvalue_2 (`self.GetDistanceTo` _returnvalue self))
  (bind _rootcomponent (`Actor.RootComponent` (`self.K2_GetPawn`)))
  (if (< _returnvalue_2 (`self.AggroDistance`))
    (`|AIMoveTo` _returnvalue (0.0 0.0 0.0) (`GameplayStatics.GetPlayerCharacter` 0)
      (:`then`
        (`FMODBlueprintStatics.PlayEventAttached` "/Game/FMOD/Events/SFX_Turtle_Steps.SFX_Turtle_Steps" _rootcomponent "None" (0.0 0.0 0.0) "SnapToTarget" true)
        (`KismetSystemLibrary.Delay` 0.2)
        (`FMODBlueprintStatics.PlayEventAttached` "/Game/FMOD/Events/SFX_Turtle_Steps.SFX_Turtle_Steps" _rootcomponent "None" (0.0 0.0 0.0) "SnapToTarget" true)))
    (else
      (`KismetSystemLibrary.PrintString` (`KismetStringLibrary.Conv_DoubleToString` _returnvalue_2)))))

(fn `UserConstructionScript`)