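; Base enemy projectile that damages the player through an interface message and destroys itself on impact.
; On sphere overlap, actors implementing BPI_Player receive DamageSubitMessage, other non-enemy actors just destroy the projectile, and BPI_Enemy actors are passed through.
; The construction script feeds ProjectileSpeed into SetSpeed, which sets both initial and max speed on the ProjectileMovement component.
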(event `self.ReceiveBeginPlay`)

(event `self.Sphere.OnComponentBeginOverlap`
  (params (OverlappedComponent :type "PrimitiveComponent Object Reference") (OtherActor :type "Actor Object Reference") (OtherComp :type "PrimitiveComponent Object Reference") (OtherBodyIndex :type Integer) (bFromSweep :type Boolean) (SweepResult :type "HitResult Structure (by ref)"))
  (if (`KismetSystemLibrary.DoesImplementInterface` OtherActor "/Game/BluePrint/BPI_Player.BPI_Player_C")
    (message `/Game/BluePrint/BPI_Player.DamageSubit` OtherActor)
    (`self.K2_DestroyActor`)
    (elif (not (`KismetSystemLibrary.DoesImplementInterface` OtherActor "/Game/BluePrint/BPI_Enemy.BPI_Enemy_C"))
      (`self.K2_DestroyActor`))))

(fn `SetSpeed`
  (params (`Projectile Speed` :type "Float (single-precision)"))
  (bind _projectilemovement (`self.ProjectileMovement`))
  (bind _output_get (set `ProjectileMovementComponent.InitialSpeed` `Projectile Speed` _projectilemovement))
  (set `ProjectileMovementComponent.MaxSpeed` _output_get _projectilemovement))

(fn `UserConstructionScript`
  (`self.SetSpeed` (`self.Projectile Speed`)))