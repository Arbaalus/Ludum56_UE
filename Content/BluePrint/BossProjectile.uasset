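; Boss projectile actor that damages the player on contact or turns into a melee enemy if it overshoots.
; A looping timer compares its distance from the instigator with the player's distance, then spawns BP_EnemyCac at its transform and destroys itself once it is farther.
; Sphere overlap sends the damage message to BPI_Player actors and destroys the projectile, which also dies on anything else not implementing BPI_Enemy.
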(event `self.ReceiveBeginPlay`
  (`parent.ReceiveBeginPlay`)
  (`KismetSystemLibrary.K2_SetTimerDelegate` (delegate `SpawnEnemyIfProjectileIsFurtherThanPlayer`) 0.3 true))

(event `SpawnEnemyIfProjectileIsFurtherThanPlayer`
  (bind _instigator (`self.Instigator`))
  (if (> (`self.GetDistanceTo` self _instigator) (`self.GetDistanceTo` _instigator (`GameplayStatics.GetPlayerCharacter` 0)))
    (`|SpawnActorFromClass` "/Game/BluePrint/BP_EnemyCac.BP_EnemyCac_C" (`self.GetTransform` self) "Undefined" "MultiplyWithRoot" null null)
    (`self.K2_DestroyActor`)))

(event `self.Sphere.OnComponentBeginOverlap`
  (params (OverlappedComponent :type "PrimitiveComponent Object Reference") (OtherActor :type "Actor Object Reference") (OtherComp :type "PrimitiveComponent Object Reference") (OtherBodyIndex :type Integer) (bFromSweep :type Boolean) (SweepResult :type "HitResult Structure (by ref)"))
  (if (`KismetSystemLibrary.DoesImplementInterface` OtherActor "/Game/BluePrint/BPI_Player.BPI_Player_C")
    (message `/Game/BluePrint/BPI_Player.DamageSubit` OtherActor)
    (`self.K2_DestroyActor`)
    (elif (not (`KismetSystemLibrary.DoesImplementInterface` OtherActor "/Game/BluePrint/BPI_Enemy.BPI_Enemy_C"))
      (`self.K2_DestroyActor`))))

(fn `UserConstructionScript`
  (`parent.UserConstructionScript`))