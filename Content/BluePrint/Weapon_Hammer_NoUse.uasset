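; Hammer weapon Blueprint, marked NoUse in its name, that plays a melee swing animation when fired.
; Shoot calls the AttackCAC event, which restarts the Attack timeline to blend the actor's pitch from the Cylinder's relative pitch toward straight down.
; Roll and yaw are preserved during the swing, and pitch resets to zero when the timeline finishes.
; It contains no hit detection or damage logic.
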(event `AttackCAC`
  (bind (_returnvalue_roll _returnvalue_pitch _returnvalue_yaw) (`KismetMathLibrary.BreakRotator` (`self.K2_GetActorRotation`)))
  (bind (_returnvalue_roll_2 _returnvalue_pitch_2 _returnvalue_yaw_2) (`KismetMathLibrary.BreakRotator` (`self.K2_GetActorRotation`)))
  (bind (_relativerotation_roll _relativerotation_pitch) (`KismetMathLibrary.BreakRotator` (`SceneComponent.RelativeRotation` (`self.Cylinder`))))
  (bind (_direction _alpha) (`Timeline|Attack` :!via `PlayFromStart`)
    (:`Update`
      (`self.K2_SetActorRotation` (`KismetMathLibrary.MakeRotator` _returnvalue_roll_2 (`KismetMathLibrary.Lerp` _relativerotation_pitch -90.0 _alpha) _returnvalue_yaw_2)))
    (:`Finished`
      (`self.K2_SetActorRotation` (`KismetMathLibrary.MakeRotator` _returnvalue_roll 0.0 _returnvalue_yaw)))))

(fn `Shoot`
  (`self.AttackCAC`))

(fn `UserConstructionScript`
  (`parent.UserConstructionScript`))