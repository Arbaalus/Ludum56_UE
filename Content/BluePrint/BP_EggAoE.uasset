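; BP_EggAoE is a short-lived area-of-effect actor for an egg attack that damages players it touches.
; On BeginPlay it plays an attached seagull sound event and starts a one-second timer that destroys it.
; Its Sphere's begin-overlap event checks the other actor for BPI_Player and sends it DamageSubitMessage, with debug prints on overlap and removal.
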(event `self.ReceiveBeginPlay`
  (`KismetSystemLibrary.K2_SetTimerDelegate` (delegate `RemoveAoE`) 1.0)
  (`FMODBlueprintStatics.PlayEventAttached` "/Game/FMOD/Events/SFX_Seagull_Shit.SFX_Seagull_Shit" (`self.DefaultSceneRoot`) "None" (0.0 0.0 0.0) "KeepRelativeOffset"))

(event `RemoveAoE`
  (`self.K2_DestroyActor`)
  (`KismetSystemLibrary.PrintString` "AoE destroyed"))

(event `self.Sphere.OnComponentBeginOverlap`
  (params (OverlappedComponent :type "PrimitiveComponent Object Reference") (OtherActor :type "Actor Object Reference") (OtherComp :type "PrimitiveComponent Object Reference") (OtherBodyIndex :type Integer) (bFromSweep :type Boolean) (SweepResult :type "HitResult Structure (by ref)"))
  (`KismetSystemLibrary.PrintString` "overlap")
  (if (`KismetSystemLibrary.DoesImplementInterface` OtherActor "/Game/BluePrint/BPI_Player.BPI_Player_C")
    (message `/Game/BluePrint/BPI_Player.DamageSubit` OtherActor)))

(fn `UserConstructionScript`)