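; Box-bounded area actor that launches timed seagull attacks across the player's surroundings, with attached audio.
; BeginPlay starts a looping timer, resettable through UpdateSeagullInterval, apparently driving StartSeagullAttack.
; Each attack spawns a numbered BP_SeagullPawn on the box's minimum-Y edge and sends it toward the opposite edge, randomizing X around the player (only the start clamps to the box).
; Leftover debug code on BeginPlay spawns a placeholder and prints positions.
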(event `self.ReceiveBeginPlay`
  (`self.TestFuncToDropAfterDev`)
  (`self.UpdateSeagullInterval` (`self.SeagullInterval`))
  (`FMODBlueprintStatics.PlayEventAttached` "/Game/FMOD/Events/SFX_Seagull_DriveBy.SFX_Seagull_DriveBy" (`self.DefaultSceneRoot`) "None" (0.0 0.0 0.0) "KeepRelativeOffset"))

(event `StartSeagullAttack`
  (bind _startattacklocation (`self.DefineAttackStartLocation`))
  (bind _attackendlocation (`self.DefineAttackEndLocation`))
  (bind _returnvalue (`|SpawnActorFromClass` "/Game/BluePrint/BP_SeagullPawn.BP_SeagullPawn_C" (`KismetMathLibrary.MakeTransform` _startattacklocation) "Undefined" "MultiplyWithRoot" null null))
  (`/Game/BluePrint/BP_SeagullPawn.SetEndLocation` _returnvalue _attackendlocation)
  (`/Game/BluePrint/BP_SeagullPawn.SetSeagullId` _returnvalue (`self.SeagullSpawnedCounter`))
  (`FMODBlueprintStatics.PlayEventAttached` "/Game/FMOD/Events/SFX_Seagull_Shit.SFX_Seagull_Shit" null "None" _startattacklocation "SnapToTarget")
  (set `self.SeagullSpawnedCounter` (+ (`self.SeagullSpawnedCounter`) 1)))

(fn `DefineAttackEndLocation`
  (returns (AttackEndLocation :type "Vector Structure"))
  (bind _seagullattackamplitude (`self.SeagullAttackAmplitude`))
  (bind (_origin _boxextent) (`KismetSystemLibrary.GetComponentBounds` (`self.Box`)))
  (bind _returnvalue_x (`KismetMathLibrary.BreakVector` (`self.K2_GetActorLocation` (`GameplayStatics.GetPlayerPawn` 0))))
  (return (`KismetMathLibrary.MakeVector` (`KismetMathLibrary.RandomFloatInRange` (- _returnvalue_x _seagullattackamplitude) (+ _returnvalue_x _seagullattackamplitude)) (+ (.y _origin) (.y _boxextent)))))

(fn `DefineAttackStartLocation`
  (returns (StartAttackLocation :type "Vector Structure"))
  (bind _seagullattackamplitude (`self.SeagullAttackAmplitude`))
  (bind (_origin _boxextent) (`KismetSystemLibrary.GetComponentBounds` (`self.Box`)))
  (bind _returnvalue_x (`KismetMathLibrary.BreakVector` (`self.K2_GetActorLocation` (`GameplayStatics.GetPlayerPawn` 0))))
  (bind (_returnvalue_x_2 _returnvalue_y _returnvalue_z) (`KismetMathLibrary.BreakVector` (`self.K2_GetActorLocation` (`GameplayStatics.GetPlayerPawn` 0))))
  (return (`KismetMathLibrary.MakeVector` (`KismetMathLibrary.RandomFloatInRange` (`KismetMathLibrary.FMax` (- _returnvalue_x _seagullattackamplitude) (- (.x _origin) (.x _boxextent))) (`KismetMathLibrary.FMin` (+ _returnvalue_x _seagullattackamplitude) (+ (.x _origin) (.x _boxextent)))) (- (.y _origin) (.y _boxextent)) _returnvalue_z)))

(fn `TestFuncToDropAfterDev`
  (bind (_origin _boxextent) (`KismetSystemLibrary.GetComponentBounds` (`self.Box`)))
  (bind _returnvalue (`|SpawnActorFromClass` "/Game/BluePrint/BP_Placeholder.BP_Placeholder_C" (`KismetMathLibrary.MakeTransform` (+ _origin _boxextent) (struct) (`KismetMathLibrary.MakeVector` 1.0 1.0 (.z _boxextent))) "Undefined" "MultiplyWithRoot" null null))
  (`KismetSystemLibrary.PrintString` (`KismetStringLibrary.Concat_StrStr` "Placeholder: " (`KismetStringLibrary.Conv_VectorToString` (`self.K2_GetActorLocation` _returnvalue))) true true (struct :`G` 0.66 :`B` 1.0 :`A` 1.0) 10.0)
  (`KismetSystemLibrary.PrintString` (`KismetStringLibrary.Concat_StrStr` "Player: " (`KismetStringLibrary.Conv_VectorToString` (`self.K2_GetActorLocation` (`GameplayStatics.GetPlayerPawn` 0)))) true true (struct :`G` 0.66 :`B` 1.0 :`A` 1.0) 10.0))

(fn `UpdateSeagullInterval`
  (params (NewSeagullInterval :type Integer))
  (if (`KismetSystemLibrary.K2_IsValidTimerHandle` (`self.SeagullAttackTimer`))
    (`KismetSystemLibrary.K2_ClearAndInvalidateTimerHandle` (`self.SeagullAttackTimer`)))
  (bind _returnvalue (`KismetSystemLibrary.K2_SetTimerDelegate` (`|CreateDelegate` :!event `StartSeagullAttack`) (`KismetMathLibrary.Conv_IntToDouble` NewSeagullInterval) true))
  (set `self.SeagullAttackTimer` _returnvalue)
  (set `self.SeagullInterval` NewSeagullInterval))

(fn `UserConstructionScript`)