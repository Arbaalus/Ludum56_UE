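; Gatling gun weapon Blueprint, a child of a parent weapon class that supplies the attack and shooting logic.
; On each attack event it sets the FMOD weapon type to the minigun sound, runs the parent attack, then rolls the tank gatling cannon component a fixed step to fake barrel spin.
; Shoot, Tick and the construction script only call their parent versions.
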(event `self.ReceiveTick`
  (params (DeltaSeconds :type "Float (single-precision)"))
  (`parent.ReceiveTick` DeltaSeconds))

(event `self.Weap_Att`
  (set `self.Fmod_WeaponType` "/Game/FMOD/Events/SFX_Minigun.SFX_Minigun")
  (`parent.Weap_Att`)
  (`SceneComponent.K2_AddLocalRotation` (`self.M_Tank__GatlingCanons`) (`KismetMathLibrary.MakeRotator` 45.0) false false))

(fn `Shoot`
  (`parent.Shoot`))

(fn `UserConstructionScript`
  (`parent.UserConstructionScript`))