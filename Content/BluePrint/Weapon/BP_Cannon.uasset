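; BP_Cannon is a cannon weapon Blueprint that fires cannonball projectiles.
; Its Attack event spawns a BP_Cannonball at the ShootDirection component's world transform, always spawning regardless of collisions and passing in ProjectileSpeed.
; The Shoot override is empty with its parent call left unconnected, so firing logic lives only in Attack.
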(event `/Game/BluePrint/Weapon/BPI_Weapon.Attack`
  (params (LoadingLaser :type "Float (double-precision)"))
  (`|SpawnActorFromClass` "/Game/BluePrint/Weapon/BP_Cannonball.BP_Cannonball_C" (`SceneComponent.K2_GetComponentToWorld` (`self.ShootDirection`)) "AlwaysSpawn" "MultiplyWithRoot" null (`self.Projectile Speed`) null))

(fn `Shoot`)

(fn `UserConstructionScript`
  (`parent.UserConstructionScript`))