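; Saw weapon Blueprint that swings through up to 180 degrees of yaw and damages enemies, mirrored by the Right flag.
; Attack is DoOnce-gated and plays the RotationSaw timeline, which rotates the root and sphere-traces at R each update, with debug drawing on.
; Hit BPI_Enemy actors take damage through the interface, tracked in EnnemlyTouch to prevent repeats.
; That list clears at a side-dependent curve value and on finish, when the attack also re-arms.
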(event `self.ReceiveBeginPlay`
  (`parent.ReceiveBeginPlay`)
  (`KismetSystemLibrary.Delay` 0.2)
  (`SceneComponent.K2_SetRelativeRotation` (`self.DefaultSceneRoot`) (* (struct :`Yaw` 180.0) (`KismetMathLibrary.SelectFloat` 1.0 0.0 (`self.Right?`))) false false))

(event `/Game/BluePrint/Weapon/BPI_Weapon.Attack`
  (params (LoadingLaser :type "Float (double-precision)"))
  (bind _returnvalue (`SceneComponent.K2_GetComponentLocation` (`self.r`)))
  (`/Engine/EditorBlueprintResources/StandardMacros.DoOnce` false :!label _label
    (:`Completed`
      (bind (_direction _01 _101) (`Timeline|rotation saw` :!via `PlayFromStart`)
        (:`Update`
          (`SceneComponent.K2_SetRelativeRotation` (`self.DefaultSceneRoot`) (* (struct :`Yaw` 180.0) (`KismetMathLibrary.SelectFloat` _101 _01 (`self.Right?`))) false false)
          (if (== _01 (`KismetMathLibrary.SelectFloat` 0.0 1.0 (`self.Right?`)))
            (`KismetArrayLibrary.Array_Clear` (`self.EnnemlyTouch`)))
          (bind _outhits (`KismetSystemLibrary.SphereTraceMulti` :`Start` _returnvalue :`End` _returnvalue :`Radius` 100.0 :`TraceChannel` "TraceTypeQuery1" :`DrawDebugType` "ForDuration" :`DrawTime` 2.0))
          (for _array_element _outhits
            (bind (_bblockinghit _binitialoverlap _time _distance _location _impactpoint _normal _impactnormal _physmat _hitactor) (`GameplayStatics.BreakHitResult` _array_element))
            (if (`KismetSystemLibrary.DoesImplementInterface` _hitactor "/Game/BluePrint/BPI_Enemy.BPI_Enemy_C")
              (if (not (`KismetArrayLibrary.Array_Contains` (`self.EnnemlyTouch`) _hitactor))
                (`KismetArrayLibrary.Array_AddUnique` (`self.EnnemlyTouch`) _hitactor)
                (message `/Game/BluePrint/BPI_Enemy.BPI_enemyTakeDamage` _hitactor 8)))))
        (:`Finished`
          (`self.reset attack`)
          (`KismetArrayLibrary.Array_Clear` (`self.EnnemlyTouch`)))))))

(event `reset attack`
  (goto _label :!via `Reset`))

(fn `UserConstructionScript`
  (`parent.UserConstructionScript`))