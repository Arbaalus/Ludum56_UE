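; Base projectile actor that damages enemies and leaves a ForceField where it hits a surface.
; A hit on Sphere spawns a scaled-up ForceField at the impact point and destroys the projectile.
; SphereCollision overlaps send WeaponDamage through BPI_Enemy, ignore BPI_Player and BPI_ProjectileSkip actors, and destroy the projectile on anything else.
; The construction script applies ProjectileSpeed as both initial and maximum movement speed.
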(event `self.ReceiveBeginPlay`)

(event `self.Sphere.OnComponentHit`
  (params (HitComponent :type "PrimitiveComponent Object Reference") (OtherActor :type "Actor Object Reference") (OtherComp :type "PrimitiveComponent Object Reference") (NormalImpulse :type "Vector Structure") (Hit :type "HitResult Structure (by ref)"))
  (`|SpawnActorFromClass` "/Game/BluePrint/Weapon/ForceField.ForceField_C" (`KismetMathLibrary.MakeTransform` (`.ImpactPoint` (`GameplayStatics.BreakHitResult` Hit)) (struct) (3.0 3.0 3.0)) "AlwaysSpawn" "MultiplyWithRoot" null null)
  (`self.K2_DestroyActor`))

(event `self.SphereCollision.OnComponentBeginOverlap`
  (params (OverlappedComponent :type "PrimitiveComponent Object Reference") (OtherActor :type "Actor Object Reference") (OtherComp :type "PrimitiveComponent Object Reference") (OtherBodyIndex :type Integer) (bFromSweep :type Boolean) (SweepResult :type "HitResult Structure (by ref)"))
  (if (`KismetSystemLibrary.DoesImplementInterface` OtherActor "/Game/BluePrint/BPI_Enemy.BPI_Enemy_C")
    (message `/Game/BluePrint/BPI_Enemy.BPI_enemyTakeDamage` OtherActor (`self.WeaponDamage`))
    (`self.K2_DestroyActor`)
    (elif (not (or (`KismetSystemLibrary.DoesImplementInterface` OtherActor "/Game/BluePrint/BPI_Player.BPI_Player_C") (`KismetSystemLibrary.DoesImplementInterface` OtherActor "/Game/BluePrint/BPI_ProjectileSkip.BPI_ProjectileSkip_C")))
      (`self.K2_DestroyActor`))))

(fn `SetSpeed`
  (params (`Projectile Speed` :type "Float (single-precision)"))
  (bind _projectilemovement (`self.ProjectileMovement`))
  (bind _output_get (set `ProjectileMovementComponent.InitialSpeed` `Projectile Speed` _projectilemovement))
  (set `ProjectileMovementComponent.MaxSpeed` _output_get _projectilemovement))

(fn `UserConstructionScript`
  (`self.SetSpeed` (`self.Projectile Speed`)))