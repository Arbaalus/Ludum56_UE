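; Base player pawn for a mech with a tank base and independently fired left and right weapons.
; On BeginPlay it adds the Enhanced Input mapping and spawns both weapons attached to MTankBase, which rotates on yaw input; movement also drives a looping-sound start/stop.
; Each attack is gated by DoOnce until that weapon's ShotDuration elapses.
; It also exposes weapon swapping, a skill tree widget, damage UI notification and keyboard spring-arm tuning with debug prints.
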(event `self.ReceiveBeginPlay`
  (bind _returnvalue (pcsubsystem `EnhancedInputLocalPlayerSubsystem` (`GameplayStatics.GetPlayerController` 0)))
  (`/Engine/EditorBlueprintResources/StandardMacros.IsValid` _returnvalue
    (:`Is Valid`
      (`EnhancedInputSubsystemInterface.AddMappingContext` _returnvalue "/Game/BluePrint/Inputs/MechaMapping.MechaMapping" 0 (struct))
      (`self.SpawnWeapon`))))

(event `EnhancedInput|/Game/BluePrint/Inputs/Move`
  (params (ActionValue :type "Vector2D Structure") (ElapsedSeconds :type "Float (double-precision)") (TriggeredSeconds :type "Float (double-precision)") (InputAction :type "InputAction Object Reference" :default "/Game/BluePrint/Inputs/Move.Move"))
  (bind (_returnvalue_roll _returnvalue_pitch _returnvalue_yaw) (`KismetMathLibrary.BreakRotator` (`self.GetControlRotation`)))
  (bind (_returnvalue_roll_2 _returnvalue_pitch_2) (`KismetMathLibrary.BreakRotator` (`self.GetControlRotation`)))
  (:`Triggered`
    (`self.AddMovementInput` (`KismetMathLibrary.GetForwardVector` (`KismetMathLibrary.MakeRotator` 0.0 0.0 _returnvalue_yaw)) ActionValue_X)
    (`self.AddMovementInput` (`KismetMathLibrary.GetRightVector` (`KismetMathLibrary.MakeRotator` 0.0 _returnvalue_pitch_2)) ActionValue_Y))
  (:`Started`
    (bind _returnvalue (`FMODBlueprintStatics.PlayEvent2D` "/Game/FMOD/Events/SFX_Player_Move.SFX_Player_Move")))
  (:`Completed`
    (`FMODBlueprintStatics.EventInstanceStop` _returnvalue)))

(event `EnhancedInput|/Game/BluePrint/Inputs/AttackLeft`
  (params (ActionValue :type Boolean) (ElapsedSeconds :type "Float (double-precision)") (TriggeredSeconds :type "Float (double-precision)") (InputAction :type "InputAction Object Reference" :default "/Game/BluePrint/Inputs/AttackLeft.AttackLeft"))
  (bind _weaponleft (`self.WeaponLeft`))
  (:`Triggered`
    (`/Engine/EditorBlueprintResources/StandardMacros.DoOnce` false :!label _label
      (:`Completed`
        (`/Engine/EditorBlueprintResources/StandardMacros.IsValid` _weaponleft
          (:`Is Valid`
            (message `/Game/BluePrint/Weapon/BPI_Weapon.Attack` _weaponleft 0.0)
            (`KismetSystemLibrary.Delay` (`/Game/BluePrint/WeaponBase.ShotDuration` _weaponleft))
            (`self.ResetShot`)))))))

(event `/Game/BluePrint/BPI_Player.DamageSubit`
  (message `/Game/BluePrint/UI/BPI_UIGame.UI_Damage` (`WidgetComponent.GetWidget` (`self.Life`))))

(event `ResetShot`
  (goto _label :!via `Reset`))

(event `EnhancedInput|/Game/BluePrint/Inputs/AttackRight`
  (params (ActionValue :type Boolean) (ElapsedSeconds :type "Float (double-precision)") (TriggeredSeconds :type "Float (double-precision)") (InputAction :type "InputAction Object Reference" :default "/Game/BluePrint/Inputs/AttackRight.AttackRight"))
  (bind _weaponright (`self.WeaponRight`))
  (:`Triggered`
    (`/Engine/EditorBlueprintResources/StandardMacros.DoOnce` false :!label _label_2
      (:`Completed`
        (`/Engine/EditorBlueprintResources/StandardMacros.IsValid` _weaponright
          (:`Is Valid`
            (message `/Game/BluePrint/Weapon/BPI_Weapon.Attack` _weaponright 0.0)
            (`KismetSystemLibrary.Delay` (`/Game/BluePrint/WeaponBase.ShotDuration` _weaponright))
            (`self.ResetShootRight`)))))))

(event `ResetShootRight`
  (goto _label_2 :!via `Reset`))

(event `Key|Add`
  (params (Key :type "Key Structure"))
  (bind _springarm (`self.SpringArm`))
  (bind _targetarmlength (`SpringArmComponent.TargetArmLength` _springarm))
  ;[1 1 1] Keyboard moveCamera
  (:`Pressed`
    (set `SpringArmComponent.TargetArmLength` (+ _targetarmlength 50.0) _springarm)
    (`KismetSystemLibrary.PrintString` (`KismetStringLibrary.Conv_DoubleToString` _targetarmlength) :!label _label_3)))

(event `Key|Subtract`
  (params (Key :type "Key Structure"))
  (bind _springarm (`self.SpringArm`))
  ;[1 1 1] Keyboard moveCamera
  (:`Pressed`
    (set `SpringArmComponent.TargetArmLength` (- (`SpringArmComponent.TargetArmLength` _springarm) 50.0) _springarm)
    (goto _label_3)))

(event `EnhancedInput|/Game/BluePrint/Inputs/RotateYaw`
  (params (ActionValue :type "Float (double-precision)") (ElapsedSeconds :type "Float (double-precision)") (TriggeredSeconds :type "Float (double-precision)") (InputAction :type "InputAction Object Reference" :default "/Game/BluePrint/Inputs/RotateYaw.RotateYaw"))
  (:`Triggered`
    (`SceneComponent.K2_AddWorldRotation` (`self.M_Tank__Base`) (`KismetMathLibrary.MakeRotator` 0.0 0.0 (* ActionValue 1.5)) false false :!label _label_4))
  (:`Completed`
    (goto _label_4)))

(event `Key|Multiply`
  (params (Key :type "Key Structure"))
  (bind _springarm (`self.SpringArm`))
  (bind _returnvalue (`SceneComponent.GetRelativeTransform` _springarm))
  ;[1 1 1] Keyboard moveCamera
  (:`Pressed`
    (`SceneComponent.K2_SetRelativeRotation` _springarm (`KismetMathLibrary.MakeRotator` 0.0 (+ (.pitch (.rotation _returnvalue)) 5.0)) false false)
    (`KismetSystemLibrary.PrintString` (`KismetStringLibrary.Conv_DoubleToString` (.pitch (.rotation _returnvalue))) :!label _label_5)))

(event `Key|NumPadNine`
  (params (Key :type "Key Structure"))
  (bind _springarm (`self.SpringArm`))
  ;[1 1 1] Keyboard moveCamera
  (:`Pressed`
    (`SceneComponent.K2_SetRelativeRotation` _springarm (`KismetMathLibrary.MakeRotator` 0.0 (- (.pitch (.rotation (`SceneComponent.GetRelativeTransform` _springarm))) 5.0)) false false)
    (goto _label_5)))

(fn `ChangeWeaponLeft`
  (params (WeaponToChange :type "/Game/BluePrint/WeaponBase Class Reference"))
  (returns (retuirn :type Boolean))
  (`self.K2_DestroyActor` (`self.WeaponLeft`))
  (bind _returnvalue (`|SpawnActorFromClass` WeaponToChange (`SceneComponent.K2_GetComponentToWorld` (`self.LocationWeaponLeft`)) "AlwaysSpawn" "MultiplyWithRoot" null null))
  (bind _output_get (set `self.WeaponLeft` _returnvalue))
  (`self.K2_AttachToComponent` _output_get (`self.M_Tank__Base`) "None" "KeepWorld" "KeepWorld" "KeepRelative" true)
  (return false))

(fn `ChangeWeaponRight`
  (params (Weapon :type "/Game/BluePrint/WeaponBase Class Reference"))
  (returns (return :type Boolean))
  (`self.K2_DestroyActor` (`self.WeaponRight`))
  (bind _returnvalue (`|SpawnActorFromClass` Weapon (`SceneComponent.K2_GetComponentToWorld` (`self.LocationWeaponRight`)) "AlwaysSpawn" "MultiplyWithRoot" null null))
  (bind _output_get (set `self.WeaponRight` _returnvalue))
  (`self.K2_AttachToComponent` _output_get (`self.M_Tank__Base`) "None" "KeepWorld" "KeepWorld" "KeepRelative" true)
  (return false))

(fn `GetWeapon`
  (returns (Left :type "/Game/BluePrint/WeaponBase Class Reference") (Right :type "/Game/BluePrint/WeaponBase Class Reference"))
  (return (`GameplayStatics.GetObjectClass` (`self.WeaponLeft`)) (`GameplayStatics.GetObjectClass` (`self.WeaponRight`))))

(fn `OpenSkillTree`
  (returns (Bool :type Boolean))
  (bind _returnvalue (`|CreateWidget` "/Game/BluePrint/UI/WBP_ArbreCompetence.WBP_ArbreCompetence_C" null (`self.LevelWeaponRange`) (`self.LevelWeaponMelee`)))
  (`UserWidget.AddToViewport` _returnvalue 0)
  (return false))

(fn `SpawnWeapon`
  (`|ExecutionSequence`
    (:`then_0`
      (bind _returnvalue (`|SpawnActorFromClass` "/Game/BluePrint/WeaponBase.WeaponBase_C" (`SceneComponent.K2_GetComponentToWorld` (`self.LocationWeaponRight`)) "AlwaysSpawn" "MultiplyWithRoot" null null))
      (bind _output_get (set `self.WeaponRight` _returnvalue))
      (`self.K2_AttachToComponent` _output_get (`self.M_Tank__Base`) "None" "KeepWorld" "KeepWorld" "KeepRelative" true))
    (:`then_1`
      (bind _returnvalue_2 (`|SpawnActorFromClass` "/Game/BluePrint/WeaponBase.WeaponBase_C" (`SceneComponent.K2_GetComponentToWorld` (`self.LocationWeaponLeft`)) "AlwaysSpawn" "MultiplyWithRoot" null null))
      (bind _output_get_2 (set `self.WeaponLeft` _returnvalue_2))
      (`self.K2_AttachToComponent` _output_get_2 (`self.M_Tank__Base`) "None" "KeepWorld" "KeepWorld" "KeepRelative" true))))

(fn `UserConstructionScript`)