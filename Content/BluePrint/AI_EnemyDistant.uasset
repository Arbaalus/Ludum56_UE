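; AI controller for a ranged-spacing enemy, apparently a turtle tank, that keeps its pawn within a distance band from the player.
; A looping half-second timer measures the distance, stepping the pawn away when too close and toward the player when too far.
; Each step is an AI MoveTo along the horizontal look-at direction, and issuing it restarts the FMOD movement sound.
; Inside the band, it issues no new move.
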(event `self.ReceiveBeginPlay`
  (`KismetSystemLibrary.K2_SetTimerDelegate` (delegate `MoveAwayFromPlayer`) 0.5 true))

(event `MoveAwayFromPlayer`
  (bind _returnvalue (`self.K2_GetPawn`))
  (bind _returnvalue_2 (`GameplayStatics.GetPlayerCharacter` 0))
  (bind _fmodaudio (`self.FMODAudio`))
  (bind _returnvalue_3 (`self.K2_GetActorLocation` _returnvalue))
  (bind _returnvalue_4 (`self.GetDistanceTo` _returnvalue _returnvalue_2))
  (bind _returnvalue_5 (`KismetMathLibrary.GetForwardVector` (`KismetMathLibrary.FindLookAtRotation` _returnvalue_3 (`self.K2_GetActorLocation` _returnvalue_2))))
  (if (< _returnvalue_4 800.0)
    (`|AIMoveTo` null (+ _returnvalue_3 (* _returnvalue_5 (-300.0 -300.0 0.0))) null
      (:`then`
        (`FMODAudioComponent.SetEvent` _fmodaudio "/Game/FMOD/Events/SFX_TurtleTank_Move.SFX_TurtleTank_Move" :!label _label)
        (`FMODAudioComponent.Play` _fmodaudio)))
    (elif (> _returnvalue_4 1500.0)
      (`|AIMoveTo` null (+ _returnvalue_3 (* _returnvalue_5 (200.0 200.0 0.0))) null
        (:`then`
          (goto _label))))))

(fn `UserConstructionScript`)