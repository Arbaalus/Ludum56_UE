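; BP_EnemyBase is an enemy base Blueprint that mostly defers to its parent class for begin play, overlap, construction and death.
; A Damage event forwards the incoming amount to TakeDamage.
; Die runs the parent logic, then removes the enemy from the SpawnedEntities list of its SpawnRef, if that reference is valid.
; Tick is disabled and test_1 is an empty event.
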(event `self.ReceiveBeginPlay`
  (`parent.ReceiveBeginPlay`))

(event `self.ReceiveActorBeginOverlap`
  (params (OtherActor :type "Actor Object Reference"))
  (`parent.ReceiveActorBeginOverlap` OtherActor))

(event `test_1`)

(event `/Game/BluePrint/BPI_Enemy.damage`
  (params (dmg :type Integer))
  (`self.TakeDamage` dmg))

(fn `Die`
  (bind _spawnref (`self.SpawnRef`))
  (`parent.Die`)
  (`/Engine/EditorBlueprintResources/StandardMacros.IsValid` _spawnref
    (:`Is Valid`
      (`KismetArrayLibrary.Array_RemoveItem` (`/Game/BluePrint/BP_BaseSpawner.SpawnedEntities` _spawnref) self))))

(fn `UserConstructionScript`
  (`parent.UserConstructionScript`))