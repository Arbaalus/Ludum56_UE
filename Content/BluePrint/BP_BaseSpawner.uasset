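; Base spawner actor that periodically spawns entities of a configurable class while the player is nearby.
; A self-recalling event loop starts on BeginPlay and attempts one spawn every Countdown seconds.
; Each spawn requires the player within range and room under MaxEntities, and lands at a random XY offset bounded by the Sphere's scaled radius.
; Spawned actors receive a SpawnRef back to the spawner and are tracked in SpawnedEntities.
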(event `SpawnLoop`
  (`self.SpawnEnemy`)
  (`KismetSystemLibrary.Delay` (`self.Countdown`))
  (`self.SpawnLoop`))

(event `self.ReceiveBeginPlay`
  (`self.SpawnLoop`))

(fn `SpawnEnemy`
  (bind (_returnvalue_location _returnvalue_rotation) (`KismetMathLibrary.BreakTransform` (`self.GetTransform` self)))
  (bind _returnvalue (`SphereComponent.GetScaledSphereRadius` (`self.Sphere`)))
  (bind _returnvalue_2 (* _returnvalue -1.0))
  (if (< (`self.GetDistanceTo` (`GameplayStatics.GetPlayerCharacter` 0)) (`self.SpawnDistanceFromPlayer`))
    (if (> (`self.MaxEntities`) (`KismetArrayLibrary.Array_Length` (`self.SpawnedEntities`)))
      (bind _returnvalue_3 (`|SpawnActorFromClass` (`self.EntityClass`) (`KismetMathLibrary.MakeTransform` (+ _returnvalue_location (`KismetMathLibrary.MakeVector` (`KismetMathLibrary.RandomFloatInRange` _returnvalue_2 _returnvalue) (`KismetMathLibrary.RandomFloatInRange` _returnvalue_2 _returnvalue))) _returnvalue_rotation) "Undefined" "MultiplyWithRoot" null null))
      (`/Engine/EditorBlueprintResources/StandardMacros.IsValid` _returnvalue_3
        (:`Is Valid`
          (set `/Game/BluePrint/BP_EnemyBase.SpawnRef` self _returnvalue_3)
          (`KismetArrayLibrary.Array_Add` (`self.SpawnedEntities`) _returnvalue_3))))))

(fn `UserConstructionScript`)