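; BP_SeagullEggActor is a seagull egg projectile that bursts into a sand explosion Niagara effect and destroys itself on actor overlap.
; SetEggId stores an identifier, which UpdateInfos prints with the egg's location.
; BeginPlay starts a looping one-second timer.
; The overlap event and the egg mesh's component-hit event print debug details of what was touched; the hit event does nothing else.
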(event `self.ReceiveBeginPlay`
  (`KismetSystemLibrary.K2_SetTimerDelegate` (`|CreateDelegate` :!event `UpdateInfos`) 1.0 true))

(event `self.ReceiveActorBeginOverlap`
  (params (OtherActor :type "Actor Object Reference"))
  (`KismetSystemLibrary.PrintString` (`KismetSystemLibrary.GetDisplayName` OtherActor) true true (struct :`R` 1.0 :`B` 0.007073 :`A` 1.0) 10.0)
  (`NiagaraFunctionLibrary.SpawnSystemAtLocation` "/Game/GameArt/FX/SYSTEMS/NS_Explosion_Sand.NS_Explosion_Sand" (`self.K2_GetActorLocation` self))
  (`self.K2_DestroyActor` self))

(event `UpdateInfos`
  (`KismetSystemLibrary.PrintString` (`KismetStringLibrary.Concat_StrStr` "Egg " (`KismetStringLibrary.Conv_IntToString` (`self.EggId`)) " Location: " (`KismetStringLibrary.Conv_VectorToString` (`self.K2_GetActorLocation` self)) " Impact point: ")))

(event `self.M_Projectiles_Oeuf.OnComponentHit`
  (params (HitComponent :type "PrimitiveComponent Object Reference") (OtherActor :type "Actor Object Reference") (OtherComp :type "PrimitiveComponent Object Reference") (NormalImpulse :type "Vector Structure") (Hit :type "HitResult Structure (by ref)"))
  (`KismetSystemLibrary.PrintString` (`KismetStringLibrary.Concat_StrStr` "Overlaped ! Source: " (`KismetSystemLibrary.GetDisplayName` HitComponent) " Other Actor: " (`KismetSystemLibrary.GetDisplayName` OtherActor) " Other Comp: " (`KismetSystemLibrary.GetDisplayName` OtherComp)) true true (struct :`R` 1.0 :`A` 1.0)))

(fn `SetEggId`
  (params (NewEggId :type Integer))
  (set `self.EggId` NewEggId))

(fn `UserConstructionScript`)